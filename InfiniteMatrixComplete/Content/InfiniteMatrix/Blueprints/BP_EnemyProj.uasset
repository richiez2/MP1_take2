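; BP_EnemyProj is an enemy projectile that reacts entirely through its actor begin-overlap event.
; Overlapping a BP_ProjectileAttack awards 20 score to the player pawn, letting the player shoot it down.
; Overlapping BP_Player reduces its health and plays a world camera shake at the player's location.
; It destroys itself on overlap with any actor, unless the player cast fails while awarding score.
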(event `self.ReceiveActorBeginOverlap`
  (params (OtherActor :type "Actor Object Reference"))
  (cast `/Game/InfiniteMatrix/Blueprints/BP_ProjectileAttack` OtherActor
    (:`then`
      (bind _asbp_player (cast `/Game/InfiniteMatrix/Blueprints/BP_Player` (`GameplayStatics.GetPlayerPawn` 0)))
      (set `/Game/InfiniteMatrix/Blueprints/BP_Player.player_score` (+ (`/Game/InfiniteMatrix/Blueprints/BP_Player.player_score` _asbp_player) 20) _asbp_player))
    (:`CastFailed`
      (bind _asbp_player_2 (cast `/Game/InfiniteMatrix/Blueprints/BP_Player` OtherActor)
        (:`then`
          (set `/Game/InfiniteMatrix/Blueprints/BP_Player.Health` (- (`/Game/InfiniteMatrix/Blueprints/BP_Player.Health` _asbp_player_2) 0.1) _asbp_player_2)
          (`GameplayStatics.PlayWorldCameraShake` "/Game/InfiniteMatrix/Blueprints/BP_CamShake.BP_CamShake_C" (`self.K2_GetActorLocation` _asbp_player_2) 0.0 1000.0))
        (:`CastFailed`
          _))))
  (`self.K2_DestroyActor`))

(fn `UserConstructionScript`)